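; Race start trigger that begins timing when a BP_vehicle06_Car overlaps it.
; It hides and teleports itself to a fixed spot, then creates a Racing_Widget, stores it in Racing_Instance and shows it.
; A Delay loop calls the widget's Timer every 0.1 seconds until the instance's Widget2 reports Finish2.
; The trigger then reappears at a lower fixed position and clears Finish2 after a short delay.
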(event OnComponentBeginOverlap(Trigger)
  (params (OverlappedComponent :type Primitive%20Component%20Object%20Reference) (OtherActor :type Actor%20Object%20Reference) (OtherComp :type Primitive%20Component%20Object%20Reference) (OtherBodyIndex :type Integer) (bFromSweep :type Boolean) (SweepResult :type Hit%20Result%20Structure%20%28by%20ref%29))
  (Utilities|Casting|CastToBP_vehicle06_Car OtherActor)
  (Rendering|SetActorHiddenInGame true)
  (Transformation|SetActorLocation "89299.000000,17200.000000,24205.000000" false true)
  (bind _returnvalue (UserInterface|CreateWidget "/Game/checkpoint_system/Racing_Widget.Racing_Widget_C"))
  (bind _asracing_instance (Utilities|Casting|CastToRacing_Instance (Game|GetGameInstance)))
  (bind _output_get (Variables|/Game/checkpoint_system/Racing_Instance.Racing_Instance_C|SetWidget _asracing_instance _returnvalue))
  (UserInterface|Viewport|AddtoViewport _returnvalue 0)
  (Default|Timer _output_get :!label _label)
  (Utilities|FlowControl|Delay 0.1)
  (if (Variables|/Game/UI/score.score_C|Getfinish2 (Variables|/Game/checkpoint_system/Racing_Instance.Racing_Instance_C|GetWidget2 _asracing_instance))
    (Rendering|SetActorHiddenInGame false)
    (Transformation|SetActorLocation "89299.000000,17200.000000,14205.000000" false true)
    (Utilities|FlowControl|Delay 5.0)
    (bind _asracing_instance_2 (Utilities|Casting|CastToRacing_Instance (Game|GetGameInstance)))
    (Variables|/Game/UI/score.score_C|Setfinish2 (Variables|/Game/checkpoint_system/Racing_Instance.Racing_Instance_C|GetWidget2 _asracing_instance_2) false)
    (else
      (goto _label))))

(event EventBeginPlay)

(event Collision|EventActorBeginOverlap
  (params (OtherActor :type Actor%20Object%20Reference)))

(event EventTick
  (params (DeltaSeconds :type Float%20%28single-precision%29)))

(fn ConstructionScript)