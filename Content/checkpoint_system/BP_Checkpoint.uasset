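; Racing checkpoint that awards points, extends the timer and moves the car's respawn point when Trigger is overlapped.
; A DoOnce gates the checkpoint and re-arms 30 seconds after Trigger2 is overlapped.
; Game Instance widgets handle score, lose check, timer and a brief "Checkpoint" message with a bell sound.
; If the Score widget flags a loss, it skips the checkpoint save and opens the menu level after a short delay.
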(event OnComponentBeginOverlap(Trigger)
  (params (OverlappedComponent :type Primitive%20Component%20Object%20Reference) (OtherActor :type Actor%20Object%20Reference) (OtherComp :type Primitive%20Component%20Object%20Reference) (OtherBodyIndex :type Integer) (bFromSweep :type Boolean) (SweepResult :type Hit%20Result%20Structure%20%28by%20ref%29))
  (Utilities|FlowControl|DoOnce false
    (:Completed
      (bind _asracing_instance (Utilities|Casting|CastToRacing_Instance (Game|GetGameInstance)))
      (Default|Puncteadd (Variables|/Game/checkpoint_system/Racing_Instance.Racing_Instance_C|GetWidget2 _asracing_instance))
      (bind _asbp_vehicle_06_car (Utilities|Casting|CastToBP_vehicle06_Car OtherActor))
      (bind _asracing_instance_2 (Utilities|Casting|CastToRacing_Instance (Game|GetGameInstance)))
      (bind _asracing_instance_3 (Utilities|Casting|CastToRacing_Instance (Game|GetGameInstance)))
      (Default|Lose1 (Variables|/Game/checkpoint_system/Racing_Instance.Racing_Instance_C|GetWidget2 _asracing_instance_3))
      (bind _foundwidgets (Widget|GetAllWidgetsOfClass "/Game/UI/score.score_C" true))
      (if (Variables|/Game/UI/score.score_C|Getlosevar (Utilities|Array|Get(acopy) _foundwidgets))
        (Utilities|FlowControl|Delay 3.0)
        (Game|OpenLevel(byName) "menu")
        (else
          (Default|TimerAdd (Variables|/Game/checkpoint_system/Racing_Instance.Racing_Instance_C|GetWidget _asracing_instance_2))
          (bind _output_get (Variables|/Game/CitySampleVehicles/vehicle06_Car/BP_vehicle06_Car.BP_vehicle06_Car_C|SetSpawn%20Position _asbp_vehicle_06_car (Transformation|GetWorldTransform (Variables|Default|GetSpawnPoint))))
          (Audio|PlaySoundatLocation "/Game/checkpoint_system/bell_sound.bell_sound" (.location _output_get) "0, 0, 0" 1.0 1.0 0.0 0 0 0 0)
          (bind _asracing_instance_4 (Utilities|Casting|CastToRacing_Instance (Game|GetGameInstance)))
          (Rendering|Components|TextRender|SetText (Variables|/Game/checkpoint_system/Racing_Widget.Racing_Widget_C|GetMessage (Variables|/Game/checkpoint_system/Racing_Instance.Racing_Instance_C|GetWidget _asracing_instance_4)) "Checkpoint")
          (Widget|SetVisibility (Variables|/Game/checkpoint_system/Racing_Widget.Racing_Widget_C|GetMessage (Variables|/Game/checkpoint_system/Racing_Instance.Racing_Instance_C|GetWidget _asracing_instance_4)) "Visible")
          (Utilities|FlowControl|Delay 1.0)
          (Widget|SetVisibility (Variables|/Game/checkpoint_system/Racing_Widget.Racing_Widget_C|GetMessage (Variables|/Game/checkpoint_system/Racing_Instance.Racing_Instance_C|GetWidget _asracing_instance_4)) "Hidden"))))))

(event OnComponentBeginOverlap(Trigger2)
  (params (OverlappedComponent :type Primitive%20Component%20Object%20Reference) (OtherActor :type Actor%20Object%20Reference) (OtherComp :type Primitive%20Component%20Object%20Reference) (OtherBodyIndex :type Integer) (bFromSweep :type Boolean) (SweepResult :type Hit%20Result%20Structure%20%28by%20ref%29))
  (Utilities|FlowControl|Delay 3e+01)
  (Utilities|FlowControl|DoOnce false) ; enters at Reset
)

(fn ConstructionScript)