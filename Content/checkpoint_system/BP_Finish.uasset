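; BP_Finish is the finish-line trigger of the checkpoint system that registers completed laps.
; When a BP_vehicle06_Car overlaps its Trigger, it calls GetFinish2 on the Racing_Instance game instance's second widget and shows a "Lap Finished" message on the first.
; After a short delay it hides the message and increments the lap number stored in the second widget.
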(event OnComponentBeginOverlap(Trigger)
  (params (OverlappedComponent :type Primitive%20Component%20Object%20Reference) (OtherActor :type Actor%20Object%20Reference) (OtherComp :type Primitive%20Component%20Object%20Reference) (OtherBodyIndex :type Integer) (bFromSweep :type Boolean) (SweepResult :type Hit%20Result%20Structure%20%28by%20ref%29))
  (Utilities|Casting|CastToBP_vehicle06_Car OtherActor)
  (bind _asracing_instance (Utilities|Casting|CastToRacing_Instance (Game|GetGameInstance)))
  (Default|GetFinish2 (Variables|/Game/checkpoint_system/Racing_Instance.Racing_Instance_C|GetWidget2 _asracing_instance))
  (Rendering|Components|TextRender|SetText (Variables|/Game/checkpoint_system/Racing_Widget.Racing_Widget_C|GetMessage (Variables|/Game/checkpoint_system/Racing_Instance.Racing_Instance_C|GetWidget _asracing_instance)) "Lap Finished")
  (Widget|SetVisibility (Variables|/Game/checkpoint_system/Racing_Widget.Racing_Widget_C|GetMessage (Variables|/Game/checkpoint_system/Racing_Instance.Racing_Instance_C|GetWidget _asracing_instance)) "Visible")
  (Utilities|FlowControl|Delay 5.0)
  (Widget|SetVisibility (Variables|/Game/checkpoint_system/Racing_Widget.Racing_Widget_C|GetMessage (Variables|/Game/checkpoint_system/Racing_Instance.Racing_Instance_C|GetWidget _asracing_instance)) "Hidden")
  (Variables|/Game/UI/score.score_C|Setlapnum (Variables|/Game/checkpoint_system/Racing_Instance.Racing_Instance_C|GetWidget2 _asracing_instance) (+ (Variables|/Game/UI/score.score_C|Getlapnum (Variables|/Game/checkpoint_system/Racing_Instance.Racing_Instance_C|GetWidget2 _asracing_instance)) 1.0)))

(event EventBeginPlay)

(event Collision|EventActorBeginOverlap
  (params (OtherActor :type Actor%20Object%20Reference)))

(event EventTick
  (params (DeltaSeconds :type Float%20%28single-precision%29)))

(fn ConstructionScript)